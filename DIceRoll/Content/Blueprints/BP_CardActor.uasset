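; Playing card actor that shows its suit and rank and has a flip event with sound.
; SetCardPicture maps Suit and Number into a dynamic material's Translation parameter to select the face, and writes the card's name to the Suitnumber text.
; FlipCard plays a sound, activates Flip and starts a Timeline after a short delay.
; The transform lerps meant to animate the flip are unwired, so they never run.
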(event Custom|FlipCard
  ;[1 1 1] Flip Card/and Sounds
  (bind _output_get (Variables|Default|SetStartPosition "0,180.000000, 0"))
  (Variables|Default|SetTempPosition (+ _output_get (Variables|/Script/Engine.SceneComponent|GetRelativeLocation (Variables|Default|GetCard))))
  (Variables|Default|SetStartRotation "180.000000, 0, 0")
  (Variables|Default|SetEndRotation "0, 0, 0")
  (Utilities|FlowControl|Sequence
    (:then_0
      (Utilities|FlowControl|Delay 0.2)
      (bind (_direction _angle _move) (Timeline|Timeline PlayFromStart)))
    (:then_1
      (Audio|PlaySoundatLocation "/Game/Cribbage_Sample/Sounds/CardFlip01_Stereo.CardFlip01_Stereo" "0, 0, 0" "0, 0, 0" 1.0 1.0 0.0 0 0 0)
      (Components|Activation|Activate (Variables|Default|GetFlip) false))))

(fn ConstructionScript)

(fn SetCardPicture
  (bind _card (Variables|Default|GetCard))
  ;[1 1 1] Function to create dynamic Material that set the picture for Card
  (bind _returnvalue (Rendering|Material|CreateDynamicMaterialInstance _card 1 0 "None" :!class /Script/Engine.PrimitiveComponent))
  (Variables|Default|SetMaterialDynamic _returnvalue)
  (Rendering|Material|SetVectorParameterValue (Variables|Default|GetMaterialDynamic) "Translation" (Math|Color|MakeColor (* (Math|Conversions|ToFloat(Integer) (Variables|Default|Getnumber)) 0.996) (Math|Conversions|ToFloat(Integer) (Variables|Default|Getsuit)) 0.0) :!class /Script/Engine.MaterialInstanceDynamic)
  (Rendering|Material|SetMaterial _card 0 (Variables|Default|GetMaterialDynamic))
  ;[1 1 1] Set Card Value and Suit
  (Utilities|FlowControl|Sequence
    (:then_0
      (switch int (Variables|Default|Getsuit)
        (:0
          (Variables|Default|Setsuit%20string " of Clubs"))
        (:1
          (Variables|Default|Setsuit%20string " of Hearts"))
        (:2
          (Variables|Default|Setsuit%20string " of Diamonds"))
        (:3
          (Variables|Default|Setsuit%20string " of Spades"))))
    (:then_1
      (switch int (Variables|Default|Getnumber)
        (:0
          (Variables|Default|Setnumber%20string "2"))
        (:1
          (Variables|Default|Setnumber%20string "3"))
        (:2
          (Variables|Default|Setnumber%20string "4"))
        (:3
          (Variables|Default|Setnumber%20string "5"))
        (:4
          (Variables|Default|Setnumber%20string "6"))
        (:5
          (Variables|Default|Setnumber%20string "7"))
        (:6
          (Variables|Default|Setnumber%20string "8"))
        (:7
          (Variables|Default|Setnumber%20string "9"))
        (:8
          (Variables|Default|Setnumber%20string "10"))
        (:9
          (Variables|Default|Setnumber%20string "Jack"))
        (:10
          (Variables|Default|Setnumber%20string "Queen"))
        (:11
          (Variables|Default|Setnumber%20string "King"))
        (:12
          (Variables|Default|Setnumber%20string "Ace"))))
    (:then_2
      (Rendering|Components|TextRender|SetText (Variables|Default|Getsuit/number) (Utilities|Text|ToText(String) (Utilities|String|Append (Variables|Default|Getnumber%20string) (Variables|Default|Getsuit%20string)))))))