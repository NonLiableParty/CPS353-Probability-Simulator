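; A physics dice actor that can be thrown and tracks which face points up.
; Each Tick transforms the local face normals to world space and stores the first one closely aligned with world up as a one-based UpFace, or zero if none qualifies.
; ThrowEvent applies an upward, mass-scaled impulse to the mesh at a random point derived from the actor bounds, so the launch can add spin.
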(event Custom|Break%20ForEachLoop
  (Utilities|Array|ForEachLoopwithBreak (Variables|Default|GetFaces%20Normals)) ; enters at Break
)

(event Custom|Throw%20Event
  (bind (_origin _boxextent) (Collision|GetActorBounds true false))
  (Physics|AddImpulseatLocation (Variables|Default|GetMesh) (* "0, 0,1.000000" (* (Physics|GetMass (Variables|Default|GetMesh)) (Variables|Default|GetLaunch%20Impulse))) (Math|Transform|TransformLocation (Transformation|GetActorTransform) (Math|Random|RandomPointinBoundingBox _origin _boxextent)) "None"))

(event EventTick
  (params (DeltaSeconds :type Float%20%28single-precision%29))
  (bind (_array_element _array_index) (Utilities|Array|ForEachLoopwithBreak (Variables|Default|GetFaces%20Normals))
    (:LoopBody
      (Variables|Default|SetUp%20Face 0)
      (if (> (Math|Vector|DotProduct (Math|Transform|TransformDirection (Transformation|GetActorTransform) _array_element) "0, 0,1.000000") 0.6)
        (Variables|Default|SetUp%20Face (+ _array_index 1))
        (CallFunction|BreakforEachLoop)))))

(fn ConstructionScript)